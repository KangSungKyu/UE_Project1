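; BP_BossGreatSword is a boss greatsword Blueprint that tracks whether its location is on the player's screen.
; Every Tick it runs CheckInViewport, which projects the actor location to screen space through player controller 0.
; The result is compared against the viewport bounds and stored in the InViewport flag; nothing in this file reads that flag.
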(event EventTick
  (params (DeltaSeconds :type Float%20%28single-precision%29))
  (Utilities|FlowControl|Sequence
    (:then_0
      (CallFunction|CheckinViewport))))

(fn ConstructionScript)

(fn CheckinViewport
  (bind _returnvalue (Game|GetPlayerController 0))
  (bind _returnvalue_2 (Transformation|GetActorLocation))
  (bind _returnvalue_3 (Viewport|GetViewportSize))
  (bind _screenlocation (Class|PlayerController|ProjectWorldLocationtoScreen _returnvalue _returnvalue_2 false))
  (Variables|Default|SetbInViewport (Math|Boolean|ANDBoolean (> (.x _screenlocation) 0.0) (> (.y _screenlocation) 0.0) (< (.x _screenlocation) (.x _returnvalue_3)) (< (.y _screenlocation) (.y _returnvalue_3))))
  (return))