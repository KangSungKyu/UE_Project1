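; Game mode that spawns players at the PlayerStart matching the level start stored in the game instance.
; Its ChoosePlayerStart override scans all PlayerStart actors and returns the first whose PlayerStartTag equals LevelStart on BP_MyGameInstance.
; Debug strings print for selected and skipped starts, and no explicit fallback handles a missing match.
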(fn ConstructionScript)

(fn ChoosePlayerStart
  (params (Player :type Controller%20Object%20Reference))
  (bind _outactors (Actor|GetAllActorsOfClass "/Script/Engine.PlayerStart"))
  (for _array_element _outactors
    (bind _asbp_my_game_instance (Utilities|Casting|CastToBP_MyGameInstance (Game|GetGameInstance)))
    (if (== (Variables|/Script/Engine.PlayerStart|GetPlayerStartTag _array_element) (Variables|/Game/Frameworks/BP_MyGameInstance.BP_MyGameInstance_C|GetLevelStart _asbp_my_game_instance))
      (Development|PrintString (Utilities|String|Append "selected start, " (Variables|/Game/Frameworks/BP_MyGameInstance.BP_MyGameInstance_C|GetLevelStart _asbp_my_game_instance)))
      (return _array_element)
      (else
        (Development|PrintString "not selected")))))