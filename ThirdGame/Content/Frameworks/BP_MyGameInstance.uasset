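; Game instance that saves and loads the player's level start tag through a single fixed save slot.
; Save writes the given level name into a BP_MySaveGame object, creating one if needed.
; Load reads the slot into LevelStart, or creates and saves a new object, then sets the first-level default in memory only after that write.
; Load prints debug messages for loaded data, created data or a failed save.
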(fn Save
  (params (LevelName :type String))
  (Utilities|IsValid (Variables|Default|GetSaveGameRef)
    (:Is%20Valid
      _)
    (:Is%20Not%20Valid
      (bind _returnvalue (SaveGame|CreateSaveGameObject "/Game/Frameworks/BP_MySaveGame.BP_MySaveGame_C"))
      (bind _output_get (Variables|Default|SetSaveGameRef _returnvalue))))
  (Variables|/Script/ThirdGame.MySaveGame|SetLevelStartTag _output_get LevelName)
  (SaveGame|SaveGametoSlot (Variables|Default|GetSaveGameRef) "TestSaveSlot"))

(fn Load
  (bind _returnvalue (SaveGame|DoesSaveGameExist "TestSaveSlot"))
  (if _returnvalue
    (bind _returnvalue_2 (SaveGame|LoadGamefromSlot "TestSaveSlot"))
    (bind _asbp_my_save_game (Utilities|Casting|CastToBP_MySaveGame _returnvalue_2))
    (bind _output_get (Variables|Default|SetSaveGameRef _asbp_my_save_game))
    (bind _output_get_2 (Variables|Default|SetLevelStart (Variables|/Script/ThirdGame.MySaveGame|GetLevelStartTag _output_get)))
    (Development|PrintString (Utilities|String|Append "load data, " _output_get_2))
    (else
      (bind _returnvalue_3 (SaveGame|CreateSaveGameObject "/Game/Frameworks/BP_MySaveGame.BP_MySaveGame_C"))
      (bind _output_get_3 (Variables|Default|SetSaveGameRef _returnvalue_3))
      (bind _returnvalue_4 (SaveGame|SaveGametoSlot _output_get_3 "TestSaveSlot"))
      (if _returnvalue_4
        (bind _output_get_4 (Variables|/Script/ThirdGame.MySaveGame|SetLevelStartTag _output_get_3 "LevelStart1"))
        (bind _output_get_5 (Variables|Default|SetLevelStart _output_get_4))
        (Development|PrintString (Utilities|String|Append "create data, " _output_get_5))
        (else
          (Development|PrintString "fail save"))))))