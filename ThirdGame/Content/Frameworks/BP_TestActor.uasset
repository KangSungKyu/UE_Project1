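; Test actor that acts as a lock-on target and periodically damages every MyCharacter in the level.
; BeginPlay creates a dynamic material on MaterialSphere and starts a looping timer that calls Damaged on those characters.
; Each Tick updates InViewport by projecting the actor's location against the viewport bounds.
; Tick also requests a red or white sphere color based on LockOned.
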(event Custom|CharacterHit_Event
  (bind _outactors (Actor|GetAllActorsOfClass "/Script/ThirdGame.MyCharacter"))
  (for _array_element _outactors
    (Class|MyCharacter|Damaged _array_element 1e+01)))

(event Custom|ChangeColor_Event
  (params (ColorValue :type Linear%20Color%20Structure))
  (bind _output_get (Variables|Default|SetColor ColorValue))
  (Rendering|Material|SetVectorParameterValue (stale EventBeginPlay _returnvalue) "Color" _output_get :!class /Script/Engine.MaterialInstanceDynamic))

(event EventTick
  (params (DeltaSeconds :type Float%20%28single-precision%29))
  (Utilities|FlowControl|Sequence
    (:then_0
      (CallFunction|CheckinViewport)
      (if (Variables|Default|GetbLockOned)
        (CallFunction|ChangeColorEvent "(R=1.000000,G=0.103198,B=0.143001,A=1.000000)")
        (else
          (CallFunction|ChangeColorEvent "(R=1.000000,G=1.000000,B=1.000000,A=1.000000)"))))))

(event EventBeginPlay
  (Utilities|FlowControl|Sequence
    (:then_0
      (bind _returnvalue (Rendering|Material|CreateDynamicMaterialInstance (Variables|Default|GetMaterialSphere) 0 0 "None" :!class /Script/Engine.PrimitiveComponent))
      (Rendering|Material|SetVectorParameterValue _returnvalue "Color" (stale Custom|ChangeColor_Event _output_get) :!class /Script/Engine.MaterialInstanceDynamic))
    (:then_1
      (Utilities|Time|SetTimerbyEvent (delegate Custom|CharacterHit_Event) 2.0 true))))

(fn ConstructionScript)

(fn CheckinViewport
  (bind _returnvalue (Game|GetPlayerController 0))
  (bind _returnvalue_2 (Transformation|GetActorLocation))
  (bind _returnvalue_3 (Viewport|GetViewportSize))
  (bind _screenlocation (Class|PlayerController|ProjectWorldLocationtoScreen _returnvalue _returnvalue_2 false))
  (Variables|Default|SetbInViewport (Math|Boolean|ANDBoolean (> (.x _screenlocation) 0.0) (> (.y _screenlocation) 0.0) (< (.x _screenlocation) (.x _returnvalue_3)) (< (.y _screenlocation) (.y _returnvalue_3))))
  (return))